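; BP_Crystal is a collectible crystal actor that flies into the player when touched and then disappears.
; On player overlap it stores its starting location, scale and point light intensity, then plays a collection timeline.
; Separate timeline tracks lerp it toward the player pawn's current position each update, shrink it to zero scale and fade its light.
; The actor destroys itself when the timeline finishes.
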(event Collision|EventActorBeginOverlap
  (params (OtherActor :type Actor%20Object%20Reference))
  (Utilities|IsPlayer OtherActor
    (:Player
      (CallFunction|StoreStartingValue)
      (bind (_direction _colletion_progers _scale_progeres _light_intensitive) (Timeline|Colletion%20Timeline Play)
        (:Update
          (CallFunction|MovetoPlayer _colletion_progers)
          (CallFunction|ToScale _scale_progeres)
          (CallFunction|AdjustLight _light_intensitive))
        (:Finished
          (Actor|DestroyActor))))))

(fn ConstructionScript)

(fn MovetoPlayer
  (params (Alpha :type Float%20%28single-precision%29))
  (Transformation|SetActorLocation (Math|Vector|Lerp(Vector) (Variables|Default|GetStartLocation) (Transformation|GetActorLocation (Game|Player|GetPlayerPawn 0)) Alpha) false false))

(fn StoreStartingValue
  (Variables|Default|SetStartLocation (Transformation|GetActorLocation))
  (Variables|Default|SetStartScale (Transformation|GetActorScale3D))
  (Variables|Default|SetStartIntensity (Variables|/Script/Engine.LightComponentBase|GetIntensity (Variables|Default|GetPointLight))))

(fn ToScale
  (params (Alpha :type Float%20%28single-precision%29))
  (Transformation|SetActorScale3D (Math|Vector|Lerp(Vector) (Variables|Default|GetStartScale) "0, 0, 0" Alpha)))

(fn AdjustLight
  (params (Alpha :type Float%20%28single-precision%29))
  (Rendering|Components|Light|SetIntensity (Variables|Default|GetPointLight) (Math|Float|Lerp (Variables|Default|GetStartIntensity) 0.0 Alpha)))