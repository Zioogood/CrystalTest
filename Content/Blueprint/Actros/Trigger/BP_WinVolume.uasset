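; BP_WinVolume is a trigger actor that ends a level when the player overlaps it.
; It blocks completion with an on-screen message while any BP_Crystal actors remain in the world.
; Otherwise it finds the current map in its LevelNames array and opens the next entry, or prints a win message and quits the game on the last one.
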(event Collision|EventActorBeginOverlap
  (params (OtherActor :type Actor%20Object%20Reference))
  (Utilities|IsPlayer OtherActor
    (:Player
      (if (CallFunction|AnyCrystalRemaining)
        (Development|PrintString "You Must  Collet All Crystal")
        (else
          (LevelManagment|CompleteLevel))))))

(fn ConstructionScript)

(fn AnyCrystalRemaining
  (bind _outactors (Actor|GetAllActorsOfClass "/Game/Blueprint/Actros/Collect/BP_Crystal.BP_Crystal_C"))
  (return (> (Utilities|Array|Length _outactors) 0)))

(fn CompleteLevel
  (if (LevelManagment|IsFinaleLevel)
    (Development|PrintString "Yea!!! You Win all Game Bravo!!")
    (Game|QuitGame 0 "Quit" false)
    (else
      (LevelManagment|LoadNextLevel))))

(fn GetCurrentLevelIndex
  (bind _returnvalue (Game|GetCurrentLevelName true))
  (return (Utilities|Array|FindItem (Variables|Default|GetLevel%20Names) (Utilities|String|StringToName _returnvalue))))

(fn IsFinaleLevel
  (return (== (Utilities|Array|LastIndex (Variables|Default|GetLevel%20Names)) (LevelManagment|GetCurrentLevelIndex))))

(fn LoadNextLevel
  (Game|OpenLevel(byName) (LevelManagment|GetNextLevelName)))

(fn GetNextLevelName
  (return (Utilities|Array|Get(acopy) (Variables|Default|GetLevel%20Names) (+ (LevelManagment|GetCurrentLevelIndex) 1))))