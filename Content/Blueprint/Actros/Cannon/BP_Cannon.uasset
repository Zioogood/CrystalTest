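; BP_Cannon is an automatic cannon actor that repeatedly fires BP_Projectile from its spawn point after a FireRate delay, starting at BeginPlay.
; Each shot spawns a projectile scaled by ProjectileScale and plays the CannonBarrleMove timeline, which slides the barrel along its relative Y axis.
; The timeline's Cannon Fire event track loops back to the delay, so the animation drives the next shot without Tick.
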(event EventBeginPlay
  (Utilities|FlowControl|Delay (Variables|Projectile|GetFireRate) :!label _label)
  (CallFunction|SpawnProjectile)
  (bind _cannon_barrel_fire (Timeline|CannonBarrleMove PlayFromStart)
    (:Update
      (CallFunction|MoveCannonBarrle _cannon_barrel_fire))
    (:Cannon_Fire
      (goto _label))))

(event Collision|EventActorBeginOverlap
  (params (OtherActor :type Actor%20Object%20Reference)))

(event EventTick
  (params (DeltaSeconds :type Float%20%28single-precision%29)))

(fn ConstructionScript)

(fn SpawnProjectile
  (bind _projectile_spawn_point (Variables|Default|GetProjectile%20Spawn%20Point))
  (Game|SpawnActorfromClass "/Game/Blueprint/Actros/Projectile/BP_Projectile.BP_Projectile_C" (Math|Transform|MakeTransform (Transformation|GetWorldLocation _projectile_spawn_point) (Transformation|GetWorldRotation _projectile_spawn_point) (Math|Conversions|ToVector(Float) (Variables|Projectile|GetProjectileScale))) "Undefined" 0 0))

(fn MoveCannonBarrle
  (params (CannonBarle_Y_Location :type Float%20%28single-precision%29))
  (Transformation|SetRelativeLocation (Variables|Default|GetCannon_Barrle) (Math|Vector|MakeVector 0.0 CannonBarle_Y_Location 0.0) false false))